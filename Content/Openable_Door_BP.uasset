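; Openable door actor that swings open and closed in response to OpenDoor interface calls.
; BeginPlay caches the starting rotation, and the DoorSwing timeline adds an animated yaw to it, playing forward on open and in reverse on close.
; Timeline event tracks play open or close sounds at the door, gated by IsOpen so each fires only in the matching direction.
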(event `self.ReceiveBeginPlay`
  (set `self.InitialRotation` (`self.K2_GetActorRotation`)))

(event `self.OpenDoor.OnOpen`
  (bind _returnvalue (`self.K2_GetActorLocation`))
  (bind _bisopen (`self.bIsOpen`))
  (set `self.bIsOpen` true)
  (bind (_direction _open_angle) (`Timeline|Door Swing` :!label _label)
    (:`Update`
      (`self.K2_SetActorRotation` (`KismetMathLibrary.ComposeRotators` (`KismetMathLibrary.MakeRotator` 0.0 0.0 _open_angle) (`self.InitialRotation`))))
    (:`Sound Open`
      (if _bisopen
        (`GameplayStatics.PlaySoundAtLocation` "/Game/door-open.door-open" _returnvalue (struct) 1.0 1.0 0.3)))
    (:`Sound Close`
      (if (not _bisopen)
        (`GameplayStatics.PlaySoundAtLocation` "/Game/door-close.door-close" _returnvalue (struct) 1.0 1.0 1.5)))))

(event `self.OpenDoor.OnClose`
  (set `self.bIsOpen` false)
  (goto _label :!via `Reverse`))

(fn `UserConstructionScript`)